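; BP_MainBody is the main body character piece, with two googly eyes animated by Control Rig.
; The construction script maps each eye's skeletal mesh to its own Control Rig component and feeds that eye's socket component into the EyeTransform control as input.
; Before each rig update, bone initial transforms are reset from the matching eye mesh.
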(event `self.ControlRig_RightEye.OnPreUpdateDelegate`
  (params (Component :type "ControlRigComponent Object Reference"))
  ;[0 0.4695 1] Set Bone Transforms for the Main Body Eyes
  (`ControlRigComponent.SetBoneInitialTransformsFromSkeletalMesh` Component (`SkinnedMeshComponent.SkeletalMesh` (`self.GooglyEyeMesh_R`))))

(event `self.ControlRig_LeftEye.OnPreUpdateDelegate`
  (params (Component :type "ControlRigComponent Object Reference"))
  ;[0 0.4695 1] Set Bone Transforms for the Main Body Eyes
  (`ControlRigComponent.SetBoneInitialTransformsFromSkeletalMesh` Component (`SkinnedMeshComponent.SkeletalMesh` (`self.GooglyEyeMesh_L`))))

(fn `UserConstructionScript`
  (`ControlRigComponent.AddMappedCompleteSkeletalMesh` (`self.ControlRig_RightEye`) (`self.GooglyEyeMesh_R`))
  (`ControlRigComponent.AddMappedElements` (`self.ControlRig_RightEye`) (`|MakeArray` (make `ControlRigComponentMappedElement` (make `ComponentReference` null "RightEyeSocket") -1 "None" "Control" "EyeTransform" "Input")))
  (`ControlRigComponent.AddMappedCompleteSkeletalMesh` (`self.ControlRig_LeftEye`) (`self.GooglyEyeMesh_L`))
  (`ControlRigComponent.AddMappedElements` (`self.ControlRig_LeftEye`) (`|MakeArray` (make `ControlRigComponentMappedElement` (make `ComponentReference` null "LeftEyeSocket") -1 "None" "Control" "EyeTransform" "Input"))))