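; BP_SwitchLevel is a level-switch actor that shows a splash screen and waits for any key to continue.
; On BeginPlay it enables input for player controller 0 and adds a WBP_Splash widget to the viewport.
; Any keyboard or gamepad key press opens the level named by its OpenLevel variable.
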(event `Key|AnyKey`
  (params (Key :type "Key Structure"))
  (:`Pressed`
    (if (`KismetInputLibrary.Key_IsKeyboardKey` Key)
      (`GameplayStatics.OpenLevel` (`self.OpenLevel`) :!label _label))))

(event `Key|AnyKey`
  (params (Key :type "Key Structure"))
  (:`Pressed`
    (if (`KismetInputLibrary.Key_IsGamepadKey` Key)
      (goto _label))))

(event `self.ReceiveBeginPlay`
  (`self.EnableInput` (`GameplayStatics.GetPlayerController` 0))
  (bind _returnvalue (`|CreateWidget` "/Game/AttachedTogether/Core/UI/WBP_Splash.WBP_Splash_C"))
  (`UserWidget.AddToViewport` _returnvalue 0))

(fn `UserConstructionScript`)